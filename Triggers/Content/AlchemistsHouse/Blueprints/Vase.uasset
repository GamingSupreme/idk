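; Vase actor in the Alchemist's House that removes potion actors from the level.
; Any overlap destroys the MyPotion1 found by class lookup, regardless of what overlapped; the preceding Item1 tag search goes unused.
; A separate custom event, not called within this graph, does the same for MyPotion5 and ignores its actor argument.
; Disconnected leftovers include destroy chains for other potions and unused Item tag checks.
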(event `self.ReceiveActorBeginOverlap`
  (params (OtherActor :type "Actor Object Reference"))
  (`GameplayStatics.GetAllActorsWithTag` "Item1")
  (bind _returnvalue (`GameplayStatics.GetActorOfClass` "/Game/AlchemistsHouse/Blueprints/MyPotion1.MyPotion1_C"))
  (`self.K2_DestroyActor` _returnvalue))

(event `CustomEvent_3`
  (params (OtherActor :type "Actor Object Reference"))
  (bind _returnvalue (`GameplayStatics.GetActorOfClass` "/Game/AlchemistsHouse/Blueprints/MyPotion5.MyPotion5_C"))
  (`self.K2_DestroyActor` _returnvalue))

(fn `UserConstructionScript`)