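; MyPotion4 is a potion actor that kills the player when it is dropped into or touches a cauldron.
; On overlap with an actor tagged Cauldron, it destroys its static mesh component and spawns an explosion effect at the player character's transform.
; After a short delay, it destroys the player character actor.
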(event `self.ReceiveActorBeginOverlap`
  (params (OtherActor :type "Actor Object Reference"))
  (if (`self.ActorHasTag` OtherActor "Cauldron")
    (`|ExecutionSequence`
      (:`then_0`
        (`ActorComponent.K2_DestroyComponent` (`self.StaticMesh`)))
      (:`then_1`
        (`|SpawnActorFromClass` "/Game/StarterContent/Blueprints/Blueprint_Effect_Explosion.Blueprint_Effect_Explosion_C" (`self.GetTransform` (`GameplayStatics.GetPlayerCharacter` 0)) "Undefined" "OverrideRootScale" null null)
        (`KismetSystemLibrary.Delay` 0.6)
        (`self.K2_DestroyActor` (`GameplayStatics.GetPlayerCharacter` 0))))))

(fn `UserConstructionScript`)